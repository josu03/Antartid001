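; Stag character Blueprint that makes the animal wander on its own, alternating movement with idle montages.
; NormalMode starts at BeginPlay, stops a montage from AnimationNormal, then uses AIMoveTo toward a random navigable point nearby.
; On arrival it shuffles AnimationNormal, plays the last element as a random pick, waits its length and calls itself again.
; Failed moves have no handler, so the loop only continues after a successful move.
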(event `self.ReceiveBeginPlay`
  (`self.NormalMode`))

(event `NormalMode`
  (bind _animationnormal (`self.AnimationNormal`))
  (for _array_element (`self.AnimationNormal`)
    _)
  (`self.StopAnimMontage` _array_element)
  (bind _randomlocation (`NavigationSystemV1.K2_GetRandomLocationInNavigableRadius` (`self.K2_GetActorLocation`) 2000.0 null null))
  (`|AIMoveTo` self _randomlocation null
    (:`OnSuccess`
      (`KismetArrayLibrary.Array_Shuffle` _animationnormal)
      (for _array_element_2 _animationnormal
        _)
      (bind _returnvalue (`self.PlayAnimMontage` _array_element_2))
      (`KismetSystemLibrary.Delay` _returnvalue)
      (`self.NormalMode`))))

(fn `UserConstructionScript`)